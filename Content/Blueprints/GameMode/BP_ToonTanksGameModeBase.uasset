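; Toon Tanks game mode Blueprint that handles the start countdown and game-over screens.
; StartGame shows the WBP_StartGame widget, and Tick maps the rounded-up remaining start time to countdown text from "Get Ready!!!" to "Go!".
; After a short delay on "Go!", it sets GameStarted and removes the widget.
; GameOver shows WBP_GameOver with a win or loss message.
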(event EventBeginPlay)

(event EventTick
  (params (DeltaSeconds :type Float%20%28single-precision%29))
  (if (not (Variables|Default|GetGameStarted))
    (bind _returnvalue (Class|ToonsTankGameModeBase|GetStartGameRemainingTime))
    (switch int (Math|Float|Ceil _returnvalue)
      (:Default
        (Rendering|Components|TextRender|SetText (Variables|/Game/Blueprints/Widgets/WBP_StartGame.WBP_StartGame_C|GetDisplayText (stale EventStartGame _returnvalue)) "Go!")
        (Utilities|FlowControl|Delay 0.5)
        (Variables|Default|SetGameStarted true)
        (Widget|RemovefromParent (stale EventStartGame _returnvalue)))
      (:1
        (Rendering|Components|TextRender|SetText (Variables|/Game/Blueprints/Widgets/WBP_StartGame.WBP_StartGame_C|GetDisplayText (stale EventStartGame _returnvalue)) "1"))
      (:2
        (Rendering|Components|TextRender|SetText (Variables|/Game/Blueprints/Widgets/WBP_StartGame.WBP_StartGame_C|GetDisplayText (stale EventStartGame _returnvalue)) "2"))
      (:3
        (Rendering|Components|TextRender|SetText (Variables|/Game/Blueprints/Widgets/WBP_StartGame.WBP_StartGame_C|GetDisplayText (stale EventStartGame _returnvalue)) "Get Ready!!!")))))

(event EventStartGame
  (bind _returnvalue (UserInterface|CreateWidget "/Game/Blueprints/Widgets/WBP_StartGame.WBP_StartGame_C"))
  (UserInterface|Viewport|AddtoViewport _returnvalue 0))

(event EventGameOver
  (params (bWonGame :type Boolean))
  (bind _returnvalue (UserInterface|CreateWidget "/Game/Blueprints/Widgets/WBP_GameOver.WBP_GameOver_C"))
  (UserInterface|Viewport|AddtoViewport _returnvalue 0)
  (Rendering|Components|TextRender|SetText (Variables|/Game/Blueprints/Widgets/WBP_GameOver.WBP_GameOver_C|GetDisplayText _returnvalue) (select bWonGame "You Won!" "You Lost!")))

(fn ConstructionScript)